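; NPC Blueprint that chases the player pawn across the navmesh while shouting random voice taunts.
; From BeginPlay, MoveNPC issues AI MoveTo toward the player's current location and re-calls itself after a short delay to keep retargeting.
; The same loop plays one of five loud positional voice cues, then uses the HasTalked flag and a longer delay as a cooldown between lines.
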(event `MoveNPC`
  (bind _returnvalue (`self.K2_GetActorLocation`))
  (bind _output_get (set `self.Location` (`SceneComponent.K2_GetComponentLocation` (`Actor.RootComponent` (`GameplayStatics.GetPlayerPawn` 0)))))
  (`|AIMoveTo` self _output_get null
    (:`then`
      (`KismetSystemLibrary.Delay` 0.1)
      (`self.MoveNPC`)
      (if (`self.hasTalked`)
        (`KismetSystemLibrary.Delay` 10.0)
        (set `self.hasTalked` false)
        (else
          (switch `int` (`KismetMathLibrary.RandomInteger` 5)
            (:`0`
              (`GameplayStatics.PlaySoundAtLocation` "/Game/Music/come_here_Cue.come_here_Cue" _returnvalue (struct) 10.0 1.0 0.0 null null null))
            (:`1`
              (`GameplayStatics.PlaySoundAtLocation` "/Game/Music/silly_child_Cue.silly_child_Cue" _returnvalue (struct) 10.0 1.0 0.0 null null null))
            (:`2`
              (`GameplayStatics.PlaySoundAtLocation` "/Game/Music/where_are_you_Cue.where_are_you_Cue" _returnvalue (struct) 10.0 1.0 0.0 null null null))
            (:`3`
              (`GameplayStatics.PlaySoundAtLocation` "/Game/Music/escape_Cue.escape_Cue" _returnvalue (struct) 10.0 1.0 0.0 null null null))
            (:`4`
              (`GameplayStatics.PlaySoundAtLocation` "/Game/Music/brat_Cue.brat_Cue" _returnvalue (struct) 10.0 1.0 0.0 null null null)))
          (set `self.hasTalked` true))))))

(event `self.ReceiveBeginPlay`
  (`self.MoveNPC`))

(fn `UserConstructionScript`)